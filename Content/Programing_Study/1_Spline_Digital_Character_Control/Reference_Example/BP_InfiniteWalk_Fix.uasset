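; Digital character actor that walks a skeletal mesh along a spline path at a configurable speed and animation rate.
; Each Tick reads the player pawn's ResetCheck and StartCheck flags to either reset or walk, so duplicated actors share one signal.
; After an optional start delay, accumulated time times WalkSpeed sets spline distance, with height and yaw offsets applied.
; Reaching the last point snaps the mesh back to the first, for open and closed splines.
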(event Custom|Walking
  (bind _spline (Variables|Default|GetSpline))
  (bind _spline_2 (Variables|Default|GetSpline))
  (bind _returnvalue (Spline|GetRotationatSplinePoint _spline_2 0 "World"))
  ;[1 1 1] 최초 출발 신호 시, Start Delay 변수의 딜레이 만큼 판단하여 시작함
  (if (!= (Variables|Setting|GetStartDelay) 0.0)
    (bind _output_get (Variables|Setting|SetStartDelayTime (+ (Variables|Setting|GetStartDelayTime) (Utilities|Time|GetWorldDeltaSeconds))))
    (if (>= _output_get (Variables|Setting|GetStartDelay))
      ;;[1 1 1] Start Delay 값 시작 후 초기화
      (Variables|Setting|SetStartDelay 0.0)
      ;[1 1 1] 디지털 캐릭터가 걷는 모션과 이동하는 로직
      ;;[1 1 1] 디지털 캐릭터 애니메이션 키 설정값 init
      (Variables|/Script/Engine.SkeletalMeshComponent|SetGlobalAnimRateScale (Variables|Default|GetSkeletalMesh) (Variables|Setting|GetAnimPlayRate) :!label _label)
      (bind _output_get_2 (Variables|Default|SetTime (+ (Variables|Default|GetTime) (Utilities|Time|GetWorldDeltaSeconds))))
      (CallFunction|SetWorldTransform _output_get_2 (Variables|Setting|GetWalkSpeed))
      (if (Math|Vector|Equal(Vector) (Spline|GetLocationatSplinePoint _spline (- (Spline|GetNumberOfSplinePoints _spline) 1) "World") (Transformation|GetWorldLocation (Variables|Default|GetSkeletalMesh)) (Variables|Setting|GetMeshHeight))
        ;[1 1 1] Spline 을 닫힌 구조로 만든 경우와 아닌 경우 판단 로직
        (if (Class|SplineComponent|IsClosedLoop (Variables|Default|GetSpline))
          ;[1 1 1] Spline 이 닫힌 구조를 경우에는 리셋시켜서 원위치에서 재출발하게 함
          (CallFunction|ResetTransform)
          (Utilities|FlowControl|Delay (Variables|Setting|GetLoopDelayDuration))
          (else
            ;[1 1 1] 최초 위치값에 디지털 캐릭터 이동시킴
            (Transformation|SetWorldTransform (Variables|Default|GetSkeletalMesh) (Math|Transform|MakeTransform (Spline|GetLocationatSplinePoint _spline_2 0 "World") (Math|Rotator|MakeRotator (.roll _returnvalue) (.pitch _returnvalue) (+ (.yaw _returnvalue) -9e+01)) "1,1,1") false false)
            (Variables|Default|SetTime 0.0)
            (Variables|Setting|SetStartDelayTime 0.0)))))
    (else
      (goto _label))))

(event EventTick
  (params (DeltaSeconds :type Float%20%28single-precision%29))
  ;[1 1 1] 움직임 판단 및 체킹, Pawn 에 제어권을 주는 이유는 액터를 복제하여 사용 시 중복처리를 줄이고 하나의 신호에 시작하기 위함
  (bind _asbp_player (Utilities|Casting|CastToBP_Player (Game|Player|GetPlayerPawn 0)))
  (Utilities|IsValid _asbp_player
    (:Is%20Valid
      (if (Variables|/Game/Programing_Study/1_Spline_Digital_Character_Control/Reference_Example/BP_Player.BP_Player_C|GetResetCheck _asbp_player)
        (CallFunction|ResetTransform)
        (elif (Variables|/Game/Programing_Study/1_Spline_Digital_Character_Control/Reference_Example/BP_Player.BP_Player_C|GetStartCheck _asbp_player)
          (CallFunction|Walking))))))

(fn ConstructionScript
  ;[1 1 1] 설정 기본값이 아닌 각각 복제한 액터의 에디터의 서로 다른 설정값의 오류를 최소화 하기 위한 방법
  (Variables|Setting|SetWalkSpeed (Variables|Setting|GetWalkSpeed))
  (Variables|Setting|SetMeshHeight (Variables|Setting|GetMeshHeight))
  (Variables|/Script/Engine.SkeletalMeshComponent|SetGlobalAnimRateScale (Variables|Default|GetSkeletalMesh) (Variables|Setting|GetAnimPlayRate))
  (Variables|Setting|SetLoopDelayDuration (Variables|Setting|GetLoopDelayDuration)))

(fn SetWorldTransform
  (params (Time :type Float%20%28single-precision%29) (Walk%20Speed :type Float%20%28single-precision%29))
  (bind _returnvalue (* Time Walk%20Speed))
  (bind _spline (Variables|Default|GetSpline))
  (bind _returnvalue_2 (Spline|GetLocationatDistanceAlongSpline _spline _returnvalue "World"))
  (bind _returnvalue_3 (Spline|GetRotationatDistanceAlongSpline _spline _returnvalue "World"))
  ;[1 1 1] Spline 을 이용한 이동 로직은 Delta Time 과 Walk Speed 변수값을 매 Tick 마다 곱해서 위치와 회전값에 Add 하는 방향으로 처리됨
  (Transformation|SetWorldTransform (Variables|Default|GetSkeletalMesh) (Math|Transform|MakeTransform (Math|Vector|MakeVector (.x _returnvalue_2) (.y _returnvalue_2) (+ (.z _returnvalue_2) (Variables|Setting|GetMeshHeight))) (Math|Rotator|MakeRotator (.roll _returnvalue_3) (.pitch _returnvalue_3) (+ (.yaw _returnvalue_3) -9e+01)) "1,1,1") false false)
  (return))

(fn ResetTransform
  (bind _spline (Variables|Default|GetSpline))
  (bind _returnvalue (Spline|GetRotationatSplinePoint _spline 0 "World"))
  (Transformation|SetWorldTransform (Variables|Default|GetSkeletalMesh) (Math|Transform|MakeTransform (Spline|GetLocationatSplinePoint _spline 0 "World") (Math|Rotator|MakeRotator (.roll _returnvalue) (.pitch _returnvalue) (+ (.yaw _returnvalue) -9e+01)) "1,1,1") false false)
  (Variables|Default|SetTime 0.0)
  (Variables|Setting|SetStartDelayTime 0.0))